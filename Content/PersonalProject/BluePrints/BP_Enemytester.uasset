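; BP_Enemytester is a test Blueprint that repeatedly damages every BP_Enemy in the level.
; From BeginPlay it gathers all enemies with GetAllActorsOfClass, then calls TakeDamage on each with a small random amount.
; It prints the enemy count, each array index and a completion message for debugging.
; After a short Delay, the GiveDamage event calls itself, forming an endless timed loop that searches again each pass.
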(event Custom|GiveDamage
  (bind _outactors (Actor|GetAllActorsOfClass "/Game/PersonalProject/BluePrints/BP_Enemy.BP_Enemy_C")) ; Find all of the enmimes
  (Development|PrintString (Utilities|String|Append "there are " (Utilities|String|ToString(Integer) (Utilities|Array|Length _outactors)) " Enemies in the level") true true "(R=0.000000,G=0.660000,B=1.000000,A=1.000000)" 5.0)
  (for (_array_element _array_index) _outactors
    (Default|TakeDamage _array_element (Math|Random|RandomFloatinRange 0.2 0.8))
    (Development|PrintString (Utilities|String|Append "Array Index  = " (Utilities|String|ToString(Integer) _array_index)) true true "(R=0.000000,G=0.660000,B=1.000000,A=1.000000)" 5.0))
  (Development|PrintString "We've Given Damage to all of the enemies" true true "(R=0.000000,G=0.660000,B=1.000000,A=1.000000)" 5.0)
  (Utilities|FlowControl|Delay 2.0)
  (CallFunction|GiveDamage))

(event EventBeginPlay
  (bind _outactors (Actor|GetAllActorsOfClass "/Game/PersonalProject/BluePrints/BP_Enemy.BP_Enemy_C")) ; Find all of the enmimes
  (Development|PrintString (Utilities|String|Append "there are " (Utilities|String|ToString(Integer) (Utilities|Array|Length _outactors)) " Enemies in the level") true true "(R=0.000000,G=0.660000,B=1.000000,A=1.000000)" 5.0)
  (for (_array_element _array_index) _outactors
    (Default|TakeDamage _array_element (Math|Random|RandomFloatinRange 0.2 0.8))
    (Development|PrintString (Utilities|String|Append "Array Index  = " (Utilities|String|ToString(Integer) _array_index)) true true "(R=0.000000,G=0.660000,B=1.000000,A=1.000000)" 5.0))
  (Development|PrintString "We've Given Damage to all of the enemies" true true "(R=0.000000,G=0.660000,B=1.000000,A=1.000000)" 5.0)
  (Utilities|FlowControl|Delay 2.0)
  (CallFunction|GiveDamage))

(fn ConstructionScript)