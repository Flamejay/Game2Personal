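; BP_Enemy is a basic enemy actor that announces itself with a printed message on BeginPlay.
; Its TakeDamage event prints a hit message and subtracts the incoming amount from Health.
; A CheckDead function tests whether Health is at or below zero, and the actor destroys itself when it returns true.
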(event Custom|TakeDamage
  (params (By%20Amount :type Float%20%28double-precision%29))
  (Development|PrintString "Ouch!!")
  (Variables|Default|Sethealth (- (Variables|Default|Gethealth) By%20Amount))
  (if (CallFunction|CheckDead (Variables|Default|Gethealth))
    (Actor|DestroyActor)))

(event EventBeginPlay
  (Development|PrintString "Hello I have been Programmed to destroy you"))

(fn ConstructionScript)

(fn CheckDead
  (params (Health :type Float%20%28double-precision%29))
  (return (<= Health 0.0)))