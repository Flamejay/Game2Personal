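; BP_Item is a base item actor that can be picked up, dropped and used.
; Pickup disables collision and physics on the Item component, then attaches to the given parent's item_socket.
; Drop detaches, restores collision and physics, and applies a fixed world-space forward and upward toss as mass-independent acceleration.
; PrimaryAction is a placeholder that only prints a debug string.
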(event Custom|Drop
  (bind _item (Variables|Default|GetItem))
  (Collision|SetCollisionEnabled (Variables|Default|GetItem) "QueryAndPhysics")
  (Transformation|DetachFromActor "KeepWorld" "KeepWorld" "KeepWorld")
  (Physics|SetSimulatePhysics _item true)
  (Physics|AddForce _item "100.000000,0.000000,250.000000" "None" true))

(event Custom|PrimaryAction
  (Development|PrintString "Calling Action"))

(event Custom|Pickup
  (params (Parent :type Scene%20Component%20Object%20Reference))
  (bind _item (Variables|Default|GetItem))
  (Collision|SetCollisionEnabled _item "NoCollision")
  (Physics|SetSimulatePhysics _item false)
  (Transformation|AttachComponentToComponent Parent "item_socket" "SnapToTarget" "SnapToTarget" "KeepRelative" true))

(event EventBeginPlay)

(event Collision|EventActorBeginOverlap
  (params (OtherActor :type Actor%20Object%20Reference)))

(event EventTick
  (params (DeltaSeconds :type Float%20%28single-precision%29)))

(fn ConstructionScript)